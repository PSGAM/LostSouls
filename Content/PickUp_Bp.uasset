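; PickUp_Bp is a pickup actor whose mesh and materials are set per instance and which can be visually highlighted.
; The construction script applies the configured static mesh and material array, turning off custom depth inside the material loop.
; A Highlight function toggles custom depth rendering on the mesh.
; The event graph holds no logic, so overlap and pickup behavior are not implemented here.
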(event EventBeginPlay)

(event Collision|EventActorBeginOverlap
  (params (OtherActor :type Actor%20Object%20Reference)))

(event EventTick
  (params (DeltaSeconds :type Float%20%28single-precision%29)))

(fn ConstructionScript
  (bind _staticmesh (Variables|Default|GetStaticMesh))
  (Components|StaticMesh|SetStaticMesh _staticmesh (Variables|Default|GetNew_StaticMesh))
  (for (_array_element _array_index) (Variables|Default|GetNew_Materials)
    (Rendering|Material|SetMaterial _staticmesh _array_index _array_element)
    (Rendering|SetRenderCustomDepth (Variables|Default|GetStaticMesh) false)))

(fn Highlight
  (params (highlight :type Boolean))
  (bind _staticmesh (Variables|Default|GetStaticMesh))
  (if highlight
    (Rendering|SetRenderCustomDepth _staticmesh true)
    (else
      (Rendering|SetRenderCustomDepth _staticmesh false))))